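; BP_PlayerController is a player controller that lets the player switch between pawns with the Tab key.
; Tab steps ControlledPawnID to the next index in the PawnsInLevel array, wrapping to the first past the end, and passes it to ControlNextPawn.
; ControlNextPawn stores that index and possesses the matching pawn.
; The graphs shown never fill PawnsInLevel or call possession on BeginPlay.
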(event Custom|ControlNextPawn
  (params (PawnID :type Integer))
  (bind _output_get (Variables|Default|SetControlledPawnID PawnID))
  (Pawn|Possess (Utilities|Array|Get(acopy) (Variables|Default|GetPawnsInLevel) _output_get)))

(event EventBeginPlay)

(event EventTick
  (params (DeltaSeconds :type Float%20%28single-precision%29)))

(event Input|KeyboardEvents|Tab
  (params (Key :type Key%20Structure :default "None"))
  (bind _controlledpawnid (Variables|Default|GetControlledPawnID))
  (bind _returnvalue (+ _controlledpawnid 1))
  (:Pressed
    (CallFunction|ControlNextPawn (Math|Integer|SelectInt 0 _returnvalue (>= _returnvalue (Utilities|Array|Length (Variables|Default|GetPawnsInLevel)))))))

(fn ConstructionScript)